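; Interactable plate that spawns an actor of RobbotClass at its Cube, staged as a teleport-in.
; Interact plays a teleport sound and a burst Niagara effect, then after a short delay swaps the burst for a scaled-up portal effect and spawns the actor with a fixed rotation.
; The portal effect is destroyed after a further delay.
; The construction script only calls its parent.
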(event EventInteract
  (bind _cube (Variables|Default|GetCube))
  (bind _returnvalue (Transformation|GetWorldLocation _cube))
  (Audio|PlaySoundatLocation "/Game/TestProject/SoundEffects/teleport.teleport" _returnvalue "0, 0, 0" 1.0 1.0 0.0 0 0 0)
  (bind _returnvalue_2 (Niagara|SpawnSystematLocation "/Game/RPGEffects/ParticlesNiagara/StatusEffects/TeleportBurst/NS_Status_Teleport_Burst.NS_Status_Teleport_Burst" (+ _returnvalue "0, 0,100.000000")))
  (Utilities|FlowControl|Delay 0.3)
  (Components|DestroyComponent _returnvalue_2)
  (bind _returnvalue_3 (Niagara|SpawnSystematLocation "/Game/RPGEffects/ParticlesNiagara/StatusEffects/TeleportPortal/NS_Status_Teleport_Portal.NS_Status_Teleport_Portal" _returnvalue "0, 0, 0" "2.000000,2.000000,2.000000"))
  (Game|SpawnActorfromClass (Variables|Default|GetRobbot%20Class) (Math|Transform|MakeTransform (.Location (Math|Transform|BreakTransform (Transformation|GetWorldTransform _cube))) "0,90.000000, 0") "Undefined" 0 0)
  (Utilities|FlowControl|Delay 2.0)
  (Components|DestroyComponent _returnvalue_3))

(fn ConstructionScript
  (|CallParentFunction))