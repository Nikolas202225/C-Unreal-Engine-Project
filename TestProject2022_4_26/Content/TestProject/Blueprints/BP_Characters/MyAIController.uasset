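; AI controller that drives a MyAIRobot pawn's movement.
; On Possess and BeginPlay it casts the controlled pawn to MyAIRobot, caches the reference and prints its display name.
; Each Tick it checks the robot's CanMove flag and, when set, calls Move with the robot's own Direction at a fixed reduced scale.
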(event EventTick
  (params (DeltaSeconds :type Float%20%28single-precision%29))
  (bind _as_my_airobot (Variables|Default|GetAs%20My%20AIRobot))
  (bind _canmove_ (Variables|/Game/TestProject/Blueprints/BP_Characters/MyAIRobot.MyAIRobot_C|GetCanMove? _as_my_airobot))
  (if _canmove_
    (Default|Move _as_my_airobot (Variables|/Game/TestProject/Blueprints/BP_Characters/MyAIRobot.MyAIRobot_C|GetDirection _as_my_airobot) 0.3 _canmove_)))

(event EventPossess
  (params (PossessedPawn :type Pawn%20Object%20Reference))
  (bind _asmy_airobot (Utilities|Casting|CastToMyAIRobot (Pawn|GetControlledPawn)))
  (bind _output_get (Variables|Default|SetAs%20My%20AIRobot _asmy_airobot))
  (Development|PrintString (Utilities|GetDisplayName _output_get)))

(event EventBeginPlay
  (bind _asmy_airobot (Utilities|Casting|CastToMyAIRobot (Pawn|GetControlledPawn)))
  (bind _output_get (Variables|Default|SetAs%20My%20AIRobot _asmy_airobot))
  (Development|PrintString (Utilities|GetDisplayName _output_get)))

(fn ConstructionScript)